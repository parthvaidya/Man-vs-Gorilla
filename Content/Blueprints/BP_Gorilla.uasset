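; Player-controlled gorilla character with Enhanced Input movement and look, a melee arm attack and a health HUD.
; Attack plays a montage gated by a DoOnce, while ToggleGorillaCollision switches the arm collider that applies damage on overlap.
; Incoming damage updates the health widget and, at zero, plays the death montage with a grunt and disables input.
; ShakeScreen triggers a world camera shake with a grunt sound.
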(event OnComponentBeginOverlap(gorillaarm)
  (params (OverlappedComponent :type Primitive%20Component%20Object%20Reference) (OtherActor :type Actor%20Object%20Reference) (OtherComp :type Primitive%20Component%20Object%20Reference) (OtherBodyIndex :type Integer) (bFromSweep :type Boolean) (SweepResult :type Hit%20Result%20Structure%20%28by%20ref%29))
  (if (not (== OtherActor self))
    (Game|Damage|ApplyDamage OtherActor 1.0 0 self)))

(event Custom|Toggle%20Gorilla%20Collision
  (params (true? :type Boolean))
  (bind _gorillaarm (Variables|Default|Getgorillaarm))
  (if true?
    (Collision|SetCollisionEnabled _gorillaarm "QueryAndPhysics")
    (else
      (Collision|SetCollisionEnabled _gorillaarm "NoCollision"))))

(event Custom|Shake%20Screen
  ;[0.15 0.15 0.15 0.5] Shake Screen
  (Camera|PlayWorldCameraShake "/Game/Blueprints/BP_CameraShake.BP_CameraShake_C" (Transformation|GetActorLocation) 0.0 1e+03)
  (Audio|PlaySoundatLocation "/Game/SFX/Gorillagrunts/SC_GoriilaGrunts.SC_GoriilaGrunts" (Transformation|GetActorLocation) "0, 0, 0" 1.0 1.0 0.0 0 0 0 0))

(event Input|EnhancedActionEvents|EnhancedInputActionIA_Move
  (params (ActionValue :type Vector%202D%20Structure) (ElapsedSeconds :type Float%20%28double-precision%29) (TriggeredSeconds :type Float%20%28double-precision%29) (InputAction :type Input%20Action%20Object%20Reference :default "/Game/Inputs/IA_Move.IA_Move"))
  (bind _returnvalue (Pawn|GetControlRotation :!class /Script/Engine.Pawn))
  ;[0.15 0.15 0.15 0.5] Add gorilla Movement to gorilla
  (Pawn|Input|AddMovementInput (Math|Vector|GetRightVector (Math|Rotator|MakeRotator (.roll _returnvalue) 0.0 (.yaw _returnvalue))) (.x ActionValue) false)
  (Pawn|Input|AddMovementInput (Math|Vector|GetForwardVector (Math|Rotator|MakeRotator 0.0 0.0 (.yaw (Pawn|GetControlRotation :!class /Script/Engine.Pawn)))) (.y ActionValue) false))

(event Input|EnhancedActionEvents|EnhancedInputActionIA_Look
  (params (ActionValue :type Vector%202D%20Structure) (ElapsedSeconds :type Float%20%28double-precision%29) (TriggeredSeconds :type Float%20%28double-precision%29) (InputAction :type Input%20Action%20Object%20Reference :default "/Game/Inputs/IA_Look.IA_Look"))
  ;[0.15 0.15 0.15 0.5] Add Look Controller
  (Pawn|Input|AddControllerYawInput (.x ActionValue))
  (Pawn|Input|AddControllerPitchInput (.y ActionValue)))

(event Input|EnhancedActionEvents|EnhancedInputActionIA_Attack
  (params (ActionValue :type Boolean) (ElapsedSeconds :type Float%20%28double-precision%29) (TriggeredSeconds :type Float%20%28double-precision%29) (InputAction :type Input%20Action%20Object%20Reference :default "/Game/Inputs/IA_Attack.IA_Attack"))
  (:Started
    (Utilities|FlowControl|DoOnce false :!label _label
      (:Completed
        (Animation|Montage|PlayMontage (Variables|Character|GetMesh) "/Game/Gorilla/Skeletal_Mesh/Animations/A_Gorillattackelftarm_Montage.A_Gorillattackelftarm_Montage" 1.7
          (:OnCompleted
            (goto _label Reset))
          (:OnInterrupted
            (goto _label Reset)))))))

(event EventBeginPlay
  (bind _returnvalue (UserInterface|CreateWidget "/Game/Widgets/WB_GorillaHealth.WB_GorillaHealth_C" 0 self))
  (bind _output_get (Variables|Default|SetGorillaHud _returnvalue))
  (UserInterface|Viewport|AddtoViewport _output_get 0)
  (Collision|SetCollisionEnabled (Variables|Default|Getgorillaarm) "NoCollision"))

(event Collision|EventActorBeginOverlap
  (params (OtherActor :type Actor%20Object%20Reference)))

(event EventTick
  (params (DeltaSeconds :type Float%20%28single-precision%29)))

(event EventPossessed
  (params (NewController :type Controller%20Object%20Reference))
  ;[0.15 0.15 0.15 0.5] Add control to gorilla
  (bind _asplayer_controller (Utilities|Casting|CastToPlayerController NewController))
  (Input|AddMappingContext (PlayerController|LocalPlayerSubsystems|GetEnhancedInputLocalPlayerSubsystem _asplayer_controller) "/Game/Inputs/IMC_Goriila.IMC_Goriila" 0 "(bIgnoreAllPressedKeysUntilRelease=True,bForceImmediately=False,bNotifyUserSettings=False)"))

(event Game|Damage|EventAnyDamage
  (params (Damage :type Float%20%28single-precision%29) (DamageType :type Damage%20Type%20Object%20Reference) (InstigatedBy :type Controller%20Object%20Reference) (DamageCauser :type Actor%20Object%20Reference))
  (bind _output_get (Variables|Default|SetHealth (- (Variables|Default|GetHealth) Damage)))
  (Default|UpdateHealthBar (Variables|Default|GetGorillaHud))
  (if (<= _output_get 0.0)
    (Utilities|FlowControl|DoOnce false
      (:Completed
        (Animation|Montage|PlayMontage (Variables|Character|GetMesh) "/Game/Gorilla/Skeletal_Mesh/Animations/A_gorriladie_Montage.A_gorriladie_Montage"
          (:then
            (Input|DisableInput (Game|GetPlayerController 0))
            (Audio|PlaySoundatLocation "/Game/SFX/Gorillagrunts/SC_GoriilaGrunts.SC_GoriilaGrunts" (Transformation|GetActorLocation) "0, 0, 0" 1.0 1.0 0.0 0 0 0 0)))))))

(fn ConstructionScript)